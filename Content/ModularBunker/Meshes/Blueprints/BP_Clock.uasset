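; BP_Clock is a clock prop in the ModularBunker set that shows the system's current time.
; Every Tick it reads Now and sets the relative pitch of separate hour, minute and second hand components.
; Each hand is angled directly from its own integer time unit, so hands move in discrete steps and the hour hand does not creep between hours.
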(event `self.ReceiveTick`
  (params (DeltaSeconds :type "Float (single-precision)"))
  (bind _returnvalue (`KismetMathLibrary.Now`))
  (`SceneComponent.K2_SetRelativeRotation` (`self.OS_ClockHours`) (`KismetMathLibrary.MakeRotator` 0.0 (`KismetMathLibrary.Conv_IntToDouble` (* (`KismetMathLibrary.GetHour12` _returnvalue) -30))) false false)
  (`SceneComponent.K2_SetRelativeRotation` (`self.OS_ClockMinutes`) (`KismetMathLibrary.MakeRotator` 0.0 (`KismetMathLibrary.Conv_IntToDouble` (* (`KismetMathLibrary.GetMinute` _returnvalue) -6))) false false)
  (`SceneComponent.K2_SetRelativeRotation` (`self.OS_ClockSeconds`) (`KismetMathLibrary.MakeRotator` 0.0 (`KismetMathLibrary.Conv_IntToDouble` (* (`KismetMathLibrary.GetSecond` _returnvalue) -6))) false false))

(fn `UserConstructionScript`)