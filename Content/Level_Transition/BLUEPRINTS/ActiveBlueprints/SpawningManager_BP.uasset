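; Spawning manager for level transitions that positions the player character and fades in the view when the level begins.
; On BeginPlay, if the save slot exists, it adds a WBP_Fade widget and reads the CustomSpawn flag from the LT_SG save.
; When the flag is set, it moves the player to a CustomSpawn_BP actor, picked at random if several exist.
; It then plays the widget's FadeOut and sets game-only input.
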(event `self.ReceiveBeginPlay`
  (bind _all_spawn_positions (`self.All Spawn Positions`))
  (bind (_returnvalue_x _returnvalue_y _returnvalue_z) (`KismetMathLibrary.BreakVector` (`self.K2_GetActorLocation` (`|GetArrayItem` (`self.All Spawn Positions`)))))
  (bind (_returnvalue_x_2 _returnvalue_y_2 _returnvalue_z_2) (`KismetMathLibrary.BreakVector` (`self.K2_GetActorLocation` (`|GetArrayItem` _all_spawn_positions (`KismetMathLibrary.RandomIntegerInRange` 0 (- (`KismetArrayLibrary.Array_Length` _all_spawn_positions) 1))))))
  ;[0 0 0] Check for SaveGame
  (bind _returnvalue (`GameplayStatics.DoesSaveGameExist` (`self.SlotName`)))
  (if _returnvalue
    ;[0 0 0] Create Widget
    (bind _returnvalue_2 (`|CreateWidget` "/Game/Level_Transition/WIDGETS/WBP_Fade.WBP_Fade_C" (`GameplayStatics.GetPlayerController` 0)))
    (`UserWidget.AddToViewport` _returnvalue_2 0)
    ;[0 0 0] Check if custom spawn should be used
    (bind _returnvalue_3 (`GameplayStatics.LoadGameFromSlot` (`self.SlotName`)))
    (bind _aslt_sg (cast `/Game/Level_Transition/BLUEPRINTS/SaveGame/LT_SG` _returnvalue_3))
    (if (`/Game/Level_Transition/BLUEPRINTS/SaveGame/LT_SG.Custom Spawn` _aslt_sg)
      ;[0 0 0] Get all possible Spawning locations
      (bind _outactors (`GameplayStatics.GetAllActorsOfClass` "/Game/Level_Transition/BLUEPRINTS/ActiveBlueprints/CustomSpawn_BP.CustomSpawn_BP_C"))
      (bind _output_get (set `self.All Spawn Positions` _outactors))
      (if (> (`KismetArrayLibrary.Array_Length` _output_get) 1)
        ;[0 0 0] Get random spawning location
        (`self.K2_SetActorLocation` (`GameplayStatics.GetPlayerCharacter` 0) (`KismetMathLibrary.MakeVector` _returnvalue_x_2 _returnvalue_y_2 _returnvalue_z_2) false false)
        (else
          ;[0 0 0] Get Spawning Point
          (`self.K2_SetActorLocation` (`GameplayStatics.GetPlayerCharacter` 0) (`KismetMathLibrary.MakeVector` _returnvalue_x _returnvalue_y _returnvalue_z) false false))))
    ;[0 0 0] Activate Fade Animation + Set Input Mode
    (`/Game/Level_Transition/WIDGETS/WBP_Fade.FadeOut` _returnvalue_2)
    (`WidgetBlueprintLibrary.SetInputMode_GameOnly` (`GameplayStatics.GetPlayerController` 0))))

(fn `UserConstructionScript`)