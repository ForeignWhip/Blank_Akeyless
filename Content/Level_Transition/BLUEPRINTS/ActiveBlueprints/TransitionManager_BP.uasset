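; Transition manager that runs a loading-screen sequence on BeginPlay, then opens the destination level stored in the LT_SG save.
; It uses the save's custom container, or randomly picks an indexed one, rerolling against and re-saving the last-used ID to avoid repeats.
; The container configures BP_RotatingActor_Updated, then fade-out, timed transition widget and fade-in play before the level opens.
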(event `self.ReceiveBeginPlay`
  (bind _returnvalue (`GameplayStatics.GetPlayerController` 0))
  ;[0 0 0] Check Custom Container
  (bind _returnvalue_2 (`GameplayStatics.LoadGameFromSlot` (`self.SlotName`)))
  (bind _aslt_sg (cast `/Game/Level_Transition/BLUEPRINTS/SaveGame/LT_SG` _returnvalue_2))
  (set `self.LoadLVL` (`/Game/Level_Transition/BLUEPRINTS/SaveGame/LT_SG.Destination Level` _aslt_sg))
  (if (`/Game/Level_Transition/BLUEPRINTS/SaveGame/LT_SG.Use Custom Container` _aslt_sg)
    ;[0 0 0] Set Custom Container
    (set `self.Selected Container` (`/Game/Level_Transition/BLUEPRINTS/SaveGame/LT_SG.Custom Container` _aslt_sg))
    (else
      ;[0 0 0] Prepare Containers (Creating Packs / Adding ID / Selecting random Container)
      (`self.Add Identificator`)
      (bind _container (`self.Load Container`))
      (set `self.Selected Container` _container)))
  ;[0 0 0] Setup the rotating actor
  (bind _returnvalue_3 (`GameplayStatics.GetActorOfClass` "/Game/Level_Transition/BLUEPRINTS/VisualBlueprints/BP_RotatingActor_Updated.BP_RotatingActor_Updated_C"))
  (`/Game/Level_Transition/BLUEPRINTS/VisualBlueprints/BP_RotatingActor_Updated.Setup Rotating Actor` _returnvalue_3 (`self.Selected Container`))
  ;[0 0 0] Play Fade Out Animation
  (bind _returnvalue_4 (`|CreateWidget` "/Game/Level_Transition/WIDGETS/WBP_Fade.WBP_Fade_C"))
  (`UserWidget.AddToViewport` _returnvalue_4 0)
  (`/Game/Level_Transition/WIDGETS/WBP_Fade.FadeOut` _returnvalue_4)
  ;[0 0 0] Create Loading Widget with Delay
  (bind _returnvalue_5 (`|CreateWidget` "/Game/Level_Transition/WIDGETS/WBP_Transition_Updated.WBP_Transition_Updated_C" _returnvalue))
  (`UserWidget.AddToViewport` _returnvalue_5 0)
  (`KismetSystemLibrary.Delay` (`/Game/Level_Transition/WIDGETS/WBP_Transition_Updated.Duration` _returnvalue_5))
  ;[0 0 0] Play Fade In Animation
  (bind _returnvalue_6 (`|CreateWidget` "/Game/Level_Transition/WIDGETS/WBP_Fade.WBP_Fade_C" _returnvalue))
  (`UserWidget.AddToViewport` _returnvalue_6 0)
  (`/Game/Level_Transition/WIDGETS/WBP_Fade.FadeIn` _returnvalue_6)
  ;[0 0 0] Open Level with Delay
  (`KismetSystemLibrary.Delay` 1.5)
  (`GameplayStatics.OpenLevel` (`self.LoadLVL`)))

(fn `Add Identificator`
  (locals (`Temp Container` :type "/Game/Level_Transition/BLUEPRINTS/Structures/Container_Package_STRUCT Structure"))
  ;[0 0 0] Creates Container Packages with container and according ID
  (`KismetArrayLibrary.Array_Clear` (`self.Container Pack`))
  (for (_array_element _array_index) (`self.Container`)
    (bind _output_get (set `local.Temp Container` (make `/Game/Level_Transition/BLUEPRINTS/Structures/Container_Package_STRUCT` _array_element _array_index)))
    (`KismetArrayLibrary.Array_Add` (`self.Container Pack`) _output_get))
  (return))

(fn `Load Container`
  (returns (Container :type "/Game/Level_Transition/BLUEPRINTS/Structures/Container_STRUCT Structure"))
  (locals (`Recheck?` :type Boolean :default true) (SaveGame :type "/Game/Level_Transition/BLUEPRINTS/SaveGame/LT_SG Object Reference") (`Last Loaded` :type Integer) (CurrentSelected :type "/Game/Level_Transition/BLUEPRINTS/Structures/Container_Package_STRUCT Structure") (`New ID` :type Integer))
  (bind _container_pack (`self.Container Pack`))
  (bind _currentselected_container (break `/Game/Level_Transition/BLUEPRINTS/Structures/Container_Package_STRUCT` (`local.CurrentSelected`)))
  ;[0 0 0] Gets the ID of the last used container
  (bind _returnvalue (`GameplayStatics.LoadGameFromSlot` (`self.SlotName`)))
  (bind _aslt_sg (cast `/Game/Level_Transition/BLUEPRINTS/SaveGame/LT_SG` _returnvalue))
  (bind _output_get (set `local.SaveGame` _aslt_sg))
  (set `local.Last Loaded` (`/Game/Level_Transition/BLUEPRINTS/SaveGame/LT_SG.Last ID` _output_get))
  ;[0 0 0] Selects random Contaier (Pack [Container / ID]) and checks if it is usable
  (while (`local.Recheck?`)
    (bind _output_get_2 (set `local.CurrentSelected` (`|GetArrayItem` _container_pack (`KismetMathLibrary.RandomIntegerInRange` 0 (- (`KismetArrayLibrary.Array_Length` _container_pack) 1)))))
    (set `local.New ID` (`.ID_5_3C2BB62F411050A98F15708D074644BF` (break `/Game/Level_Transition/BLUEPRINTS/Structures/Container_Package_STRUCT` _output_get_2)))
    (set `local.Recheck?` (== (`.ID_5_3C2BB62F411050A98F15708D074644BF` (break `/Game/Level_Transition/BLUEPRINTS/Structures/Container_Package_STRUCT` _output_get_2)) (`local.Last Loaded`))))
  ;[0 0 0] Saves ID of last used container pack to SaveGame
  (set `local.Recheck?` true)
  (bind _returnvalue_2 (`GameplayStatics.LoadGameFromSlot` (`self.SlotName`)))
  (bind _aslt_sg_2 (cast `/Game/Level_Transition/BLUEPRINTS/SaveGame/LT_SG` _returnvalue_2))
  (bind _returnvalue_3 (`GameplayStatics.CreateSaveGameObject` "/Game/Level_Transition/BLUEPRINTS/SaveGame/LT_SG.LT_SG_C"))
  (set `/Game/Level_Transition/BLUEPRINTS/SaveGame/LT_SG.Custom Spawn` (`/Game/Level_Transition/BLUEPRINTS/SaveGame/LT_SG.Custom Spawn` _aslt_sg_2) _returnvalue_3)
  (set `/Game/Level_Transition/BLUEPRINTS/SaveGame/LT_SG.Destination Level` (`/Game/Level_Transition/BLUEPRINTS/SaveGame/LT_SG.Destination Level` _aslt_sg_2) _returnvalue_3)
  (set `/Game/Level_Transition/BLUEPRINTS/SaveGame/LT_SG.Last ID` (`local.New ID`) _returnvalue_3)
  (set `/Game/Level_Transition/BLUEPRINTS/SaveGame/LT_SG.Use Custom Container` (`/Game/Level_Transition/BLUEPRINTS/SaveGame/LT_SG.Use Custom Container` _aslt_sg_2) _returnvalue_3)
  (set `/Game/Level_Transition/BLUEPRINTS/SaveGame/LT_SG.Custom Container` (`/Game/Level_Transition/BLUEPRINTS/SaveGame/LT_SG.Custom Container` _aslt_sg_2) _returnvalue_3)
  (`GameplayStatics.SaveGameToSlot` _returnvalue_3 (`self.SlotName`))
  ;[0 0 0] Returns Container out of Container Pack
  (return _currentselected_container))

(fn `UserConstructionScript`)