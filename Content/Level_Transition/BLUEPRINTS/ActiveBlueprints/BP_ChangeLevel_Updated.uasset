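; Level change trigger that starts a transition when player character 0 overlaps its box.
; It writes the destination level, custom spawn and custom container settings to an LT_SG save game, creating one if the slot is empty.
; Once the async save completes, it plays the WBP_Fade fade-in and, after a short delay, opens Level_Transition_Updated as an intermediate level, with the save carrying the destination.
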(event `self.Box.OnComponentBeginOverlap`
  (params (OverlappedComponent :type "PrimitiveComponent Object Reference") (OtherActor :type "Actor Object Reference") (OtherComp :type "PrimitiveComponent Object Reference") (OtherBodyIndex :type Integer) (bFromSweep :type Boolean) (SweepResult :type "HitResult Structure (by ref)"))
  ;[0 0 0] Checking if Player Character Overlapped
  (if (== OtherActor (`GameplayStatics.GetPlayerCharacter` 0))
    ;[0 0 0] Check for a SaveGame
    (bind _returnvalue (`GameplayStatics.DoesSaveGameExist` (`self.SlotName`)))
    (if _returnvalue
      ;[0 0 0] Save to existing SaveGame
      (bind _returnvalue_2 (`GameplayStatics.LoadGameFromSlot` (`self.SlotName`)))
      (bind _aslt_sg (cast `/Game/Level_Transition/BLUEPRINTS/SaveGame/LT_SG` _returnvalue_2))
      (set `/Game/Level_Transition/BLUEPRINTS/SaveGame/LT_SG.Destination Level` (`self.Destination Level`) _aslt_sg)
      (set `/Game/Level_Transition/BLUEPRINTS/SaveGame/LT_SG.Custom Spawn` (`self.Use Custom Spawn?`) _aslt_sg)
      (set `/Game/Level_Transition/BLUEPRINTS/SaveGame/LT_SG.Last ID` (`/Game/Level_Transition/BLUEPRINTS/SaveGame/LT_SG.Last ID` _aslt_sg) _aslt_sg)
      (set `/Game/Level_Transition/BLUEPRINTS/SaveGame/LT_SG.Use Custom Container` (`self.Load Custom Container`) _aslt_sg)
      (set `/Game/Level_Transition/BLUEPRINTS/SaveGame/LT_SG.Custom Container` (`self.Custom Container`) _aslt_sg)
      (`AsyncActionHandleSaveGame.AsyncSaveGameToSlot` _aslt_sg (`self.SlotName`)
        (:`Completed`
          _))
      (else
        ;[0 0 0] Create new Savegame
        (bind _returnvalue_3 (`GameplayStatics.CreateSaveGameObject` "/Game/Level_Transition/BLUEPRINTS/SaveGame/LT_SG.LT_SG_C"))
        (bind _output_get (set `self.Save Game Inscance` _returnvalue_3))
        (set `/Game/Level_Transition/BLUEPRINTS/SaveGame/LT_SG.Destination Level` (`self.Destination Level`) _output_get)
        (set `/Game/Level_Transition/BLUEPRINTS/SaveGame/LT_SG.Custom Spawn` (`self.Use Custom Spawn?`) _output_get)
        (set `/Game/Level_Transition/BLUEPRINTS/SaveGame/LT_SG.Use Custom Container` (`self.Load Custom Container`) _output_get)
        (set `/Game/Level_Transition/BLUEPRINTS/SaveGame/LT_SG.Custom Container` (`self.Custom Container`) _output_get)
        (`AsyncActionHandleSaveGame.AsyncSaveGameToSlot` _output_get (`self.SlotName`)
          (:`Completed`
            _))))
    ;[0 0 0] Play Fade In Animation
    (bind _returnvalue_4 (`|CreateWidget` "/Game/Level_Transition/WIDGETS/WBP_Fade.WBP_Fade_C" (`GameplayStatics.GetPlayerController` 0)))
    (`UserWidget.AddToViewport` _returnvalue_4 0)
    (`/Game/Level_Transition/WIDGETS/WBP_Fade.FadeIn` _returnvalue_4)
    ;[0 0 0] Open Transition Level with Delay
    (`KismetSystemLibrary.Delay` 1.5)
    (`GameplayStatics.OpenLevel` "Level_Transition_Updated")))

(fn `UserConstructionScript`)