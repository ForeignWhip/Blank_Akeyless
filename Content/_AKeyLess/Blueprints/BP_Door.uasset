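; BP_Door is a door that swings open and closed around its vertical axis.
; It caches the mesh's world rotation at BeginPlay as the closed pose.
; OpenDoor plays a timeline whose ZAxis track supplies a yaw offset combined with that starting rotation, and CloseDoor reverses the same timeline.
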(event `self.ReceiveBeginPlay`
  (set `self.DefaultRotation` (`SceneComponent.K2_GetComponentRotation` (`self.StaticMeshComponent`))))

(event `Open Door`
  (bind (_direction _zaxis) (`Timeline|Door Move Timeline` :!label _label)
    (:`Update`
      (`SceneComponent.K2_SetWorldRotation` (`self.StaticMeshComponent`) (`KismetMathLibrary.ComposeRotators` (`KismetMathLibrary.MakeRotator` 0.0 0.0 _zaxis) (`self.DefaultRotation`)) false false))))

(event `Close Door`
  (goto _label :!via `Reverse`))

(fn `UserConstructionScript`)