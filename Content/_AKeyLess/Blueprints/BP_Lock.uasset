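; BP_Lock is a three-dial combination lock puzzle that opens or closes a linked door.
; InteractwithPuzzle rotates the given dial's pitch left or right by a fixed step, then updates that dial's text to show its pitch.
; CheckCode compares the dial's pitch to its code entry within a small tolerance and stores the result per dial.
; The door opens when all stored results pass and closes otherwise.
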(event `/Game/_AKeyLess/Blueprints/BPI_InteractWithPuzzle.Interact with Puzzle`
  (params (Component :type "PrimitiveComponent Object Reference") (RotateLeft :type Boolean))
  (`self.Rotate` Component RotateLeft))

(fn `CheckCode`
  (params (Component :type "PrimitiveComponent Object Reference"))
  (locals (SelectedMesh :type Integer) (LocalFailed :type Boolean))
  (bind (_relativerotation_roll _relativerotation_pitch) (`KismetMathLibrary.BreakRotator` (`SceneComponent.RelativeRotation` Component)))
  (bind _doortoopen (`self.DoorToOpen`))
  (if (== Component (`self.00_Lock`))
    (set `local.SelectedMesh` 0)
    (`KismetArrayLibrary.Array_Set` (`self.CodeIsGood`) (`local.SelectedMesh`) (`KismetMathLibrary.NearlyEqual_FloatFloat` (`|GetArrayItem` (`self.Code`) (`local.SelectedMesh`)) _relativerotation_pitch 0.1) :!label _label)
    (for _array_element (`self.CodeIsGood`)
      (if (not _array_element)
        (set `local.LocalFailed` true)
        (break)))
    (if (`local.LocalFailed`)
      (`/Game/_AKeyLess/Blueprints/BP_Door.Close Door` _doortoopen)
      (else
        (`/Game/_AKeyLess/Blueprints/BP_Door.Open Door` _doortoopen)))
    (elif (== Component (`self.01_Lock`))
      (set `local.SelectedMesh` 1)
      (goto _label)
      (elif (== Component (`self.02_lock`))
        (set `local.SelectedMesh` 2)
        (goto _label)))))

(fn `Rotate`
  (params (Component :type "PrimitiveComponent Object Reference") (RotateLeft :type Boolean))
  (if RotateLeft
    (`SceneComponent.K2_AddRelativeRotation` Component (`KismetMathLibrary.MakeRotator` 0.0 (* (`self.RotateValue`) -1.0)) false false)
    (else
      (`SceneComponent.K2_AddRelativeRotation` Component (`KismetMathLibrary.MakeRotator` 0.0 (`self.RotateValue`)) false false)))
  (`KismetSystemLibrary.PrintString` (`KismetStringLibrary.Conv_RotatorToString` (`SceneComponent.RelativeRotation` Component)))
  (`self.Set Display Number` Component)
  (`self.CheckCode` Component))

(fn `Set Display Number`
  (params (Component_SM :type "PrimitiveComponent Object Reference"))
  (bind _01_lock (`self.01_Lock`))
  (bind _00_lock (`self.00_Lock`))
  (bind _02_lock (`self.02_lock`))
  (bind (_relativerotation_roll _relativerotation_pitch) (`KismetMathLibrary.BreakRotator` (`SceneComponent.RelativeRotation` _02_lock)))
  (bind (_relativerotation_roll_2 _relativerotation_pitch_2) (`KismetMathLibrary.BreakRotator` (`SceneComponent.RelativeRotation` _00_lock)))
  (bind (_relativerotation_roll_3 _relativerotation_pitch_3) (`KismetMathLibrary.BreakRotator` (`SceneComponent.RelativeRotation` _01_lock)))
  ;[1 0.1647 0] Setting 00 Lock Display Text
  (if (== Component_SM _00_lock)
    (`TextRenderComponent.K2_SetText` (`self.00_ Number`) (`KismetTextLibrary.Conv_DoubleToText` _relativerotation_pitch_2 "HalfToEven"))
    (else
      ;[1 0.1647 0] Setting 01 Lock Display Text
      (if (== Component_SM _01_lock)
        (`TextRenderComponent.K2_SetText` (`self.00_ Number1`) (`KismetTextLibrary.Conv_DoubleToText` _relativerotation_pitch_3 "HalfToEven"))
        (else
          ;[1 0.1647 0] Setting 02 Lock Display Text
          (if (== Component_SM _02_lock)
            (`TextRenderComponent.K2_SetText` (`self.00_ Number2`) (`KismetTextLibrary.Conv_DoubleToText` _relativerotation_pitch "HalfToEven"))))))))

(fn `UserConstructionScript`)