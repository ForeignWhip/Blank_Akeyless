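; Game mode for the Akeyless level that tracks how many Talkables remain and ends the game when none are left.
; Talkables register and report interactions, adjusting a counter that is broadcast through the TalkableAmountUpdated dispatcher.
; BeginPlay forces low scalability settings via console commands and creates the HUD widget.
; At zero, it disables player input, plays a congratulations sound, shows the end screen and blocks pausing.
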(event `TalkableRegister`
  ;[1 1 1] Call Dispatcher when Talkables are created
  (bind _result (`/Engine/EditorBlueprintResources/StandardMacros.IncrementInt` (`self.TalkablesLeft`))
    (:`  `
      (`self.TalkableAmountUpdated` _result))))

(event `TalkableInteracted`
  ;[1 1 1] Call Dispatcher when Talkables are interacted with
  (bind _result (`/Engine/EditorBlueprintResources/StandardMacros.DecrementInt` (`self.TalkablesLeft`))
    (:`  `
      (`self.TalkableAmountUpdated` _result))))

(event `self.ReceiveBeginPlay`
  ;[1 1 1] Setting Graphics
  (`KismetSystemLibrary.ExecuteConsoleCommand` "sg.PostProcessQuality 1" null)
  (`KismetSystemLibrary.ExecuteConsoleCommand` "sg.ViewDistanceQuality 1" null)
  (`KismetSystemLibrary.ExecuteConsoleCommand` "sg.AntiAliasingQuality 1" null)
  (`KismetSystemLibrary.ExecuteConsoleCommand` "sg.ResolutionQuality 50" null)
  (`KismetSystemLibrary.ExecuteConsoleCommand` "sg.ShadowQuality 1" null)
  (`KismetSystemLibrary.ExecuteConsoleCommand` "sg.GlobalIlluminationQuality 1" null)
  (`KismetSystemLibrary.ExecuteConsoleCommand` "sg.ReflectionQuality 1" null)
  (`KismetSystemLibrary.ExecuteConsoleCommand` "sg.TextureQuality 1" null)
  (`KismetSystemLibrary.ExecuteConsoleCommand` "sg.EffectsQuality 1" null)
  (`KismetSystemLibrary.ExecuteConsoleCommand` "sg.FoliageQuality 1" null)
  (`KismetSystemLibrary.ExecuteConsoleCommand` "sg.ShadingQuality 1" null)
  ;[1 1 1] Assigning Event Dispatcher and Creating Widget
  (add `self.TalkableAmountUpdated` (delegate `TalkableAmountUpdated_Event`))
  (bind _returnvalue (`|CreateWidget` "/Game/_AKeyLess/UI/UI_Akeyless.UI_Akeyless_C"))
  (`UserWidget.AddToViewport` _returnvalue 0))

(event `TalkableAmountUpdated_Event` :!signature `self.TalkableAmountUpdated`
  (params (Count :type Integer))
  (bind _returnvalue (`GameplayStatics.GetPlayerController` 0))
  ;[1 1 1] Assigning Event Dispatcher and Creating Widget
  (if (<= Count 0)
    (`self.DisableInput` _returnvalue null)
    (`GameplayStatics.PlaySound2D` "/Game/_AKeyLess/Audio/AudioFiles/04_CongratsEnd.04_CongratsEnd" 1.0 1.0 0.0 null null)
    (bind _returnvalue_2 (`|CreateWidget` "/Game/_AKeyLess/UI/UI_EndScreen.UI_EndScreen_C" _returnvalue))
    (`UserWidget.AddToViewport` _returnvalue_2 0)
    (`WidgetBlueprintLibrary.SetInputMode_GameAndUIEx` _returnvalue _returnvalue_2)
    (bind _asbp_first_person_character (cast `/Game/FirstPerson/Blueprints/BP_FirstPersonCharacter` (`GameplayStatics.GetPlayerCharacter` 0)))
    (set `/Game/FirstPerson/Blueprints/BP_FirstPersonCharacter.CanPause` false _asbp_first_person_character)))

(fn `UserConstructionScript`)