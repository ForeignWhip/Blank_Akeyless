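; Shelf actor that checks whether a bottle placed on it matches the shelf's color, apparently for a color-matching puzzle.
; When a BP_Bottle overlaps ShelfCollision, its color is compared to ShelfColor within a small tolerance, setting IsColorCorrect.
; A match also fires CorrectLightEvent on the first BP_ColorCheckerLight found in the level.
; No end-overlap logic clears the flag, and a physics-disable node is left unconnected.
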(event `self.ShelfCollision.OnComponentBeginOverlap`
  (params (OverlappedComponent :type "PrimitiveComponent Object Reference") (OtherActor :type "Actor Object Reference") (OtherComp :type "PrimitiveComponent Object Reference") (OtherBodyIndex :type Integer) (bFromSweep :type Boolean) (SweepResult :type "HitResult Structure (by ref)"))
  (if (`KismetMathLibrary.ClassIsChildOf` (`GameplayStatics.GetObjectClass` OtherActor) "/Game/_AKeyLess/Blueprints/BP_Bottle.BP_Bottle_C")
    (bind _asbp_bottle (cast `/Game/_AKeyLess/Blueprints/BP_Bottle` OtherActor))
    (if (`KismetMathLibrary.LinearColor_IsNearEqual` (`KismetMathLibrary.Conv_ColorToLinearColor` (`/Game/_AKeyLess/Blueprints/BP_Bottle.Bottle Color` _asbp_bottle)) (`KismetMathLibrary.Conv_ColorToLinearColor` (`self.ShelfColor`)) 0.1)
      (set `self.IsColorCorrect` true)
      (bind _returnvalue (`GameplayStatics.GetActorOfClass` "/Game/_AKeyLess/Blueprints/BP_ColorCheckerLight.BP_ColorCheckerLight_C"))
      (`/Game/_AKeyLess/Blueprints/BP_ColorCheckerLight.CorrectLightEvent` _returnvalue)
      (else
        (set `self.IsColorCorrect` false)))))

(fn `UserConstructionScript`)