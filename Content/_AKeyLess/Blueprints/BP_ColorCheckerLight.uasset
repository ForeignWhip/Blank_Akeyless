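; BP_ColorCheckerLight is a puzzle feedback light that turns two rect lights green once a correct-light event has fired three times.
; Each CorrectLightEvent call increments a Ticker counter and recolors RectLight and RectLight1 when it reaches exactly three.
; Tick prints the counter to screen every frame as debug output.
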(event `CorrectLightEvent`
  (set `self.Ticker` (+ (`self.Ticker`) 1.0))
  (if (== (`self.Ticker`) 3.0)
    (`LightComponent.SetLightColor` (`self.RectLight`) (struct :`R` 0.038528 :`G` 1.0 :`A` 1.0) true)
    (`LightComponent.SetLightColor` (`self.RectLight1`) (struct :`R` 0.038528 :`G` 1.0 :`A` 1.0) true)))

(event `self.ReceiveTick`
  (params (DeltaSeconds :type "Float (single-precision)"))
  (`KismetSystemLibrary.PrintString` (`KismetStringLibrary.Conv_DoubleToString` (`self.Ticker`)) true true (struct :`G` 0.66 :`B` 1.0 :`A` 1.0) 2.0 "Key"))

(fn `UserConstructionScript`)