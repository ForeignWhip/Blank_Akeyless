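; BP_Elevator is a one-way elevator that the player starts by pressing the pickup input inside its trigger box.
; Box overlap enables or disables input and, until first use, toggles the interact prompt.
; Activation turns the button blue and runs a DoOnce-gated timeline that lerps the root from its BeginPlay height to TargetZ, disabling player input as it moves.
; An alternate timeline-driven movement path is left unused.
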(event `self.ReceiveBeginPlay`
  ;[0.6355 0 1] Storing the initial World Location
  (set `self.InitialLocation` (`SceneComponent.K2_GetComponentLocation` (`self.DefaultSceneRoot`))))

(event `self.BoxCollision.OnComponentBeginOverlap`
  (params (OverlappedComponent :type "PrimitiveComponent Object Reference") (OtherActor :type "Actor Object Reference") (OtherComp :type "PrimitiveComponent Object Reference") (OtherBodyIndex :type Integer) (bFromSweep :type Boolean) (SweepResult :type "HitResult Structure (by ref)"))
  ;[1 0.2078 0] Enable Input when the user is close enough to start the elevator
  (if (== OtherActor (`GameplayStatics.GetPlayerCharacter` 0))
    (`self.EnableInput` (`GameplayStatics.GetPlayerController` 0))
    (if (not (`self.ElevatorUsed`))
      (`SceneComponent.ToggleVisibility` (`self.Interact Text`) false))))

(event `self.BoxCollision.OnComponentEndOverlap`
  (params (OverlappedComponent :type "PrimitiveComponent Object Reference") (OtherActor :type "Actor Object Reference") (OtherComp :type "PrimitiveComponent Object Reference") (OtherBodyIndex :type Integer))
  ;[1 0.2078 0] Disable Input when the user exits the BoxCollision
  (if (== OtherActor (`GameplayStatics.GetPlayerCharacter` 0))
    (`self.DisableInput` (`GameplayStatics.GetPlayerController` 0))
    (if (not (`self.ElevatorUsed`))
      (`SceneComponent.ToggleVisibility` (`self.Interact Text`) false))))

(event `InputAction|Input_Pickup`
  (params (Key :type "Key Structure"))
  ;[1 0.2078 0] Start the Elevator when the user presses E
  (:`Pressed`
    (`self.ActivateElevator`)
    (`SceneComponent.ToggleVisibility` (`self.Interact Text`) false)
    (set `self.ElevatorUsed` true)
    (`PrimitiveComponent.SetMaterial` (`self.Button`) 0 "/Game/LevelPrototyping/Materials/MI_Solid_Blue.MI_Solid_Blue")))

(event `ActivateElevator`
  (bind (_initiallocation_x _initiallocation_y _initiallocation_z) (`KismetMathLibrary.BreakVector` (`self.InitialLocation`)))
  ;[1 0.2078 0] Logic for moving the Elevator
  (`/Engine/EditorBlueprintResources/StandardMacros.DoOnce` false
    (:`Completed`
      (bind (_direction _alpha) (`Timeline|MoveUpAlpha`)
        (:`Update`
          (`SceneComponent.K2_SetWorldLocation` (`self.DefaultSceneRoot`) (`KismetMathLibrary.MakeVector` _initiallocation_x _initiallocation_y (`KismetMathLibrary.Lerp` _initiallocation_z (`self.TargetZ`) _alpha)) false false)
          (`self.DisableInput` (`GameplayStatics.GetPlayerController` 0)))))))

(fn `UserConstructionScript`)