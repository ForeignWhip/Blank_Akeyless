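; Elevator actor that raises itself once when the player character enters its trigger box.
; BeginPlay stores the starting location, then the first player overlap plays a timeline that lerps the root's world Z to TargetZ, keeping X and Y fixed.
; A DoOnce with no reset makes the ride one-way.
; An unconnected older branch that sets Z directly from a MoveUp timeline never runs.
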(event `self.ReceiveBeginPlay`
  (set `self.InitialLocation` (`SceneComponent.K2_GetComponentLocation` (`self.DefaultSceneRoot`))))

(event `self.BoxCollision.OnComponentBeginOverlap`
  (params (OverlappedComponent :type "PrimitiveComponent Object Reference") (OtherActor :type "Actor Object Reference") (OtherComp :type "PrimitiveComponent Object Reference") (OtherBodyIndex :type Integer) (bFromSweep :type Boolean) (SweepResult :type "HitResult Structure (by ref)"))
  (bind (_initiallocation_x _initiallocation_y _initiallocation_z) (`KismetMathLibrary.BreakVector` (`self.InitialLocation`)))
  (if (== OtherActor (`GameplayStatics.GetPlayerCharacter` 0))
    (`/Engine/EditorBlueprintResources/StandardMacros.DoOnce` false
      (:`Completed`
        (bind (_direction _alpha) (`Timeline|MoveUpAlpha`)
          (:`Update`
            (`SceneComponent.K2_SetWorldLocation` (`self.DefaultSceneRoot`) (`KismetMathLibrary.MakeVector` _initiallocation_x _initiallocation_y (`KismetMathLibrary.Lerp` _initiallocation_z (`self.TargetZ`) _alpha)) false false)))))))

(fn `UserConstructionScript`)